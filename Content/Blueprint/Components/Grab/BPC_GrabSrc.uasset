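; Actor component that acts as the grabbing side of a grab system, paired with BPC_GrabTar components on target actors.
; Grab finds the first tag-matched target component, binds a success event and requests a grab with a duration.
; Successful grabs are recorded in an actor-to-component map, which ReleaseActor and ReleaseAll use to release targets and remove their entries.
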(event EventBeginPlay)

(event EventTick
  (params (DeltaSeconds :type Float%20%28single-precision%29)))

(fn Grab
  (params (GrabTargetActor :type Actor%20Object%20Reference) (Duration :type Float%20%28single-precision%29) (MatchTag :type Name))
  (Utilities|IsValid GrabTargetActor
    (:Is%20Valid
      (bind _output_get (LocalVariables|SetTargetComp (Utilities|Array|Get(acopy) (Actor|GetComponentsbyTag GrabTargetActor "/InteractionFramework/Blueprint/Components/Grab/BPC_GrabTar.BPC_GrabTar_C" MatchTag))))
      (Utilities|IsValid _output_get
        (:Is%20Valid
          (EventDispatchers|BindEventtoOnGrabSuccess _output_get (EventDispatchers|CreateEvent :!event OnGrabSuccess))
          (bind _success (Default|BeGrab _output_get self Duration))
          (return _success))
        (:Is%20Not%20Valid
          (return false))))))

(fn OnGrabSuccess
  (params (TargetComp :type BPC%20Grab%20Tar%20Object%20Reference))
  (Utilities|Map|Add (Variables|Default|GetGrabActors) (Components|GetOwner TargetComp) TargetComp))

(fn ReleaseActor
  (params (Actor :type Actor%20Object%20Reference))
  (bind _grabactors (Variables|Default|GetGrabActors))
  (bind (_value _returnvalue) (Utilities|Map|Find _grabactors Actor))
  (if _returnvalue
    (Default|BeRelease _value)
    (Utilities|Map|Remove (Variables|Default|GetGrabActors) Actor)
    (return true)))

(fn ReleaseAll
  (bind _keys (Utilities|Map|Keys (Variables|Default|GetGrabActors)))
  (for _array_element _keys
    (CallFunction|ReleaseActor _array_element))
  (Utilities|Map|Clear (Variables|Default|GetGrabActors)))