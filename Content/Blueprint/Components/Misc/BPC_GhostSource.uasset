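; Scene component that spawns a BP_GhostHelper for its owner and sends that ghost to other actors.
; GhostToActor picks the target actor's BPC_GhostTarget nearest this component, makes the ghost opaque and records its starting transform.
; Tick linearly eases the ghost to that target over the given duration, or jumps when it is not positive, then attaches it.
; GhostToActorByTag and GhostToPoint are empty stubs.
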(event EventBeginPlay
  (bind _returnvalue (Components|GetOwner))
  (bind _returnvalue_2 (Game|SpawnActorfromClass "/InteractionFramework/Blueprint/Helper/BP_GhostHelper.BP_GhostHelper_C" (Transformation|GetActorTransform _returnvalue) "Undefined" _returnvalue (Variables|Default|GetDraw%20Debug) 0))
  (Default|InitGhostHelper _returnvalue_2 _returnvalue)
  (Variables|Default|SetGhostHelper _returnvalue_2))

(event EventTick
  (params (DeltaSeconds :type Float%20%28single-precision%29))
  (Variables|Default|SetDelta%20Seconds DeltaSeconds)
  (if (Variables|Default|GetbFlyTo)
    (bind _targetcomp (Variables|Default|GetTargetComp)
      (:then
        (bind _ghosthelper (Variables|Default|GetGhostHelper)
          (:then
            (if (> (Variables|Default|GetDuration) 0.0)
              (Variables|Default|SetAlpha (+ (Variables|Default|GetAlpha) (/ (Variables|Default|GetDelta%20Seconds) (Variables|Default|GetDuration))))
              (Transformation|SetActorTransform _ghosthelper (Math|Interpolation|Ease "Linear" (Variables|Default|GetAlpha) (Variables|Default|GetStartGhostHelprTrans) (Transformation|GetWorldTransform _targetcomp)))
              (if (>= (Variables|Default|GetAlpha) 1.0)
                (Variables|Default|SetbFlyTo false :!label _label)
                (Transformation|AttachComponentToComponent _ghosthelper (Variables|Default|GetTargetComp) "None" "SnapToTarget" "SnapToTarget" "SnapToTarget" true)
                (Variables|Default|SetAlpha 0.0))
              (else
                (Transformation|SetActorTransform _ghosthelper (Transformation|GetWorldTransform _targetcomp))
                (goto _label))))
          (:else)))
      (:else))))

(fn GhosttoActor
  (params (TargetActor :type Actor%20Object%20Reference) (Duration :type Float%20%28single-precision%29))
  (bind _output_get (LocalVariables|SetTargetComps (Actor|GetComponentsByClass TargetActor "/InteractionFramework/Blueprint/Components/Misc/BPC_GhostTarget.BPC_GhostTarget_C")))
  (bind _output_get_2 (Variables|Default|SetTargetComp (CallFunction|GetNearestComp _output_get)))
  (Utilities|IsValid _output_get_2
    (:Is%20Valid
      (Variables|Default|SetDuration Duration)
      (Variables|Default|SetbFlyTo true)
      (bind _ghosthelper (Variables|Default|GetGhostHelper)
        (:then
          (Default|SetGhostOpacity _ghosthelper 1.0)
          (Variables|Default|SetStartGhostHelprTrans (Transformation|GetActorTransform _ghosthelper))
          (return true))
        (:else)))))

(fn GhosttoActorbyTag)

(fn GhosttoPoint)

(fn GetNearestComp
  (params (Comps :type Array%20of%20BPC%20Ghost%20Target%20Object%20References))
  (LocalVariables|Setdist 9999999.0)
  (if (== (Utilities|Array|Length Comps) 0)
    (return (Utilities|Array|Get(acopy) Comps))
    (else
      (for _array_element Comps
        (if (< (Class|KismetMathLibrary|VectorDistanceSquared (Transformation|GetWorldLocation _array_element) (Transformation|GetWorldLocation)) (LocalVariables|Getdist))
          (LocalVariables|Setdist (Class|KismetMathLibrary|VectorDistanceSquared (Transformation|GetWorldLocation _array_element) (Transformation|GetWorldLocation)))
          (LocalVariables|SetnearestComp _array_element)))
      (return (LocalVariables|GetnearestComp)))))