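; VR player movement component that gives its owning Character walk and jump actions.
; DoWalk feeds the movement component an input vector along the forward vector of the direction component held in WalkData, scaled by the input value.
; DoJump prints a leftover "Hello" debug string and calls Jump on the owning Character.
; BeginPlay caches the owner as a Character, and Tick is empty.
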(event EventBeginPlay
  (bind _ascharacter (Utilities|Casting|CastToCharacter (Components|GetOwner))))

(event EventTick
  (params (DeltaSeconds :type Float%20%28single-precision%29)))

(event EventDoWalk
  (params (Value :type Float%20%28single-precision%29))
  (bind _aspawn_movement_component (Utilities|Casting|CastToPawnMovementComponent (Variables|Default|GetMovementComponent)))
  (Class|PawnMovementComponent|AddInputVector _aspawn_movement_component (* (Math|Vector|GetForwardVector (.directioncomponent (Variables|Default|GetWalkData))) Value) false))

(event EventDoJump
  (params (Value :type Float%20%28single-precision%29))
  (Development|PrintString "Hello")
  (bind _ascharacter (Utilities|Casting|CastToCharacter (Components|GetOwner)))
  (Character|Jump _ascharacter))