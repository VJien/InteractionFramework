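; IF_PreView_Hand is a helper actor that previews a VR hand pose, with all its logic in the construction script.
; It mirrors the Hand mesh on Y for left hands and toggles between a ghost and a basic hand material.
; Finger data comes from the DT_HandPose row matching HandPoseKey, falling back to HandPoseData, and is pushed into the ABP_IF_VR_Hand anim instance.
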(event EventBeginPlay)

(event Collision|EventActorBeginOverlap
  (params (OtherActor :type Actor%20Object%20Reference)))

(event EventTick
  (params (DeltaSeconds :type Float%20%28single-precision%29)))

(fn ConstructionScript
  (bind _hand (Variables|Default|GetHand))
  (Utilities|FlowControl|Sequence
    (:then_0
      (if (Variables|Default|GetbRightHand)
        (Transformation|SetRelativeScale3D _hand (Math|Vector|MakeVector 1.0 1.0 1.0))
        (else
          (Transformation|SetRelativeScale3D _hand (Math|Vector|MakeVector 1.0 -1.0 1.0)))))
    (:then_1
      (bind _returnvalue (Utilities|GetDataTableRow "/InteractionFramework/Blueprint/Data/DT_HandPose.DT_HandPose" (Variables|Default|GetHandPoseKey))
        (:then
          (Default|UpdateFingerData (CallFunction|GetAnimIns) _returnvalue))
        (:RowNotFound
          (Default|UpdateFingerData (CallFunction|GetAnimIns) (Variables|Default|GetHand%20Pose%20Data)))))
    (:then_2
      (Rendering|Material|SetMaterial (Variables|Default|GetHand) 0 (select (Variables|Default|GetbUseGhostMaterial) "/InteractionFramework/Mat/M_IF_Ghost_Inst.M_IF_Ghost_Inst" "/InteractionFramework/Asset/Hand/Materials/Mi_BasicHand_01.Mi_BasicHand_01")))))

(fn GetAnimIns
  (bind _asabp_if_vr_hand (Utilities|Casting|CastToABP_IF_VR_Hand (Components|SkeletalMesh|GetAnimInstance (Variables|Default|GetHand))))
  (return _asabp_if_vr_hand))