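; IFBP_VR_Hand is a VR hand Blueprint that drives finger and hand poses on an IFBP_VR_HandMesh child actor.
; Construction and BeginPlay set up the mesh for hand and HMD type, then apply the default table pose, falling back to default pose data.
; Wrapper functions forward pose updates and expose the mesh's aim arrow.
; Pose data table rows supply whole-hand or per-finger poses, and two rows can be lerped per finger.
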(event EventBeginPlay
  (Hand|Base|InitHandMesh))

(event EventTick
  (params (DeltaSeconds :type Float%20%28single-precision%29)))

(fn ConstructionScript
  (Hand|Base|InitHandMesh))

(fn GetAimComponent
  (bind _asifbp_vr_hand_mesh (Utilities|Casting|CastToIFBP_VR_HandMesh (Variables|/Script/Engine.ChildActorComponent|GetChildActor (Variables|Default|GetIF_VR_HandMesh))))
  (return (Variables|/InteractionFramework/Blueprint/VR/IFBP_VR_HandMesh.IFBP_VR_HandMesh_C|GetAimArrow _asifbp_vr_hand_mesh)))

(fn UpdateHandPose
  (params (Data :type IF%20VR%20Hand%20Pose%20Data%20Structure))
  (bind _asifbp_vr_hand_mesh (Utilities|Casting|CastToIFBP_VR_HandMesh (Variables|/Script/Engine.ChildActorComponent|GetChildActor (Variables|Default|GetIF_VR_HandMesh))))
  (Default|UpdateHandPose _asifbp_vr_hand_mesh Data))

(fn UpdateFingerPose
  (params (Data :type IF%20VR%20Hand%20Finger%20Data%20Structure) (Finger :type EIF_HandFingerType%20Enum :default "None"))
  (bind _asifbp_vr_hand_mesh (Utilities|Casting|CastToIFBP_VR_HandMesh (Variables|/Script/Engine.ChildActorComponent|GetChildActor (Variables|Default|GetIF_VR_HandMesh))))
  (Default|UpdateFingerPose _asifbp_vr_hand_mesh Data Finger))

(fn UpdatePosebyTable
  (params (RowName :type Name))
  (bind _returnvalue (Utilities|GetDataTableRow (Variables|Config|GetPoseDataTable) RowName)
    (:then
      (Hand|Pose|UpdateHandPose _returnvalue)
      (return true))
    (:RowNotFound
      (return false))))

(fn UpdateFingerbyTable
  (params (RowName :type Name) (Finger :type EIF_HandFingerType%20Enum :default "None"))
  (bind _returnvalue (Utilities|GetDataTableRow (Variables|Config|GetPoseDataTable) RowName)
    (:then
      (Hand|Pose|UpdateFingerPose (Utilities|Select :Index (.Index (Utilities|Struct|BreakIF_VRHandPoseData _returnvalue)) :None "" :Thumbstick (.Thumbstick (Utilities|Struct|BreakIF_VRHandPoseData _returnvalue)) :Middle (.Middle (Utilities|Struct|BreakIF_VRHandPoseData _returnvalue)) :Ring (.Ring (Utilities|Struct|BreakIF_VRHandPoseData _returnvalue)) :Pinky (.Pinky (Utilities|Struct|BreakIF_VRHandPoseData _returnvalue)) :Index Finger) Finger))))

(fn InitHandMesh
  (bind _asifbp_vr_hand_mesh (Utilities|Casting|CastToIFBP_VR_HandMesh (Variables|/Script/Engine.ChildActorComponent|GetChildActor (Variables|Default|GetIF_VR_HandMesh))))
  (Default|UpdateDefaultPoseifHMDorHandChange _asifbp_vr_hand_mesh (Variables|Config|GetHandType) (Variables|Config|GetHMD%20Type) (Variables|Config|GetPreview%20Device%20Mesh))
  (bind _success (Hand|Pose|UpdatePosebyTable (Variables|Config|GetDefaultPoseKey)))
  (if (not _success)
    (Hand|Pose|UpdateHandPose (Variables|Config|GetDefaultPoseData))))

(fn GetFingerDatabyTwoTables
  (params (TableA :type Name) (TableB :type Name) (Finger :type EIF_HandFingerType%20Enum :default "None") (Alpha :type Float%20%28single-precision%29))
  (bind _returnvalue (Utilities|GetDataTableRow (Variables|Config|GetPoseDataTable) TableA)
    (:then
      (bind _returnvalue_2 (Utilities|GetDataTableRow (Variables|Config|GetPoseDataTable) TableB)
        (:then
          (return (Class|IFBlueprintLibrary|LerpFingerData (Class|IFBlueprintLibrary|GetFingerData _returnvalue Finger) (Class|IFBlueprintLibrary|GetFingerData _returnvalue_2 Finger) Alpha)))))))

(fn UpdateMultiFingersPose
  (params (Finger :type Map%20of%20EIF_HandFingerType%20Enums%20to%20Structs :default "None"))
  (bind _asifbp_vr_hand_mesh (Utilities|Casting|CastToIFBP_VR_HandMesh (Variables|/Script/Engine.ChildActorComponent|GetChildActor (Variables|Default|GetIF_VR_HandMesh))))
  (Default|UpdateMultiFingersPose _asifbp_vr_hand_mesh Finger))