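; VR hand actor that serves as either left or right hand, with a grab source component and optional Oculus Touch controller preview meshes.
; The construction script uses HandType to mirror one hand mesh on Y, apply per-side offsets and grab rotation, and set controller visibility.
; Finger poses from DT_HandPose feed ABP_VR_Hand through SetFingerData.
; BeginPlay runs a timed, apparently test, sequence through two table poses, then enables pose mode with an idle animation.
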(event EventBeginPlay
  (bind _asabp_vr_hand (CallFunction|GetHandAnimInstance))
  (Utilities|FlowControl|Delay 0.5)
  (bind _returnvalue (Utilities|GetDataTableRow "/InteractionFramework/Blueprint/Data/DT_HandPose.DT_HandPose" "Grab_Axe")
    (:then
      (CallFunction|SetFingerData _returnvalue)
      (Utilities|FlowControl|Delay 1.0)
      (bind _returnvalue_2 (Utilities|GetDataTableRow "/InteractionFramework/Blueprint/Data/DT_HandPose.DT_HandPose" "Point")
        (:then
          (CallFunction|SetFingerData _returnvalue_2)
          (Utilities|FlowControl|Delay 1.0)
          (Default|SetPoseMode _asabp_vr_hand true)
          (Default|UpdateHandAnimation _asabp_vr_hand "/InteractionFramework/Asset/Hand/Animation/Anim_Quest_Idle.Anim_Quest_Idle"))))))

(event Collision|EventActorBeginOverlap
  (params (OtherActor :type Actor%20Object%20Reference)))

(event EventTick
  (params (DeltaSeconds :type Float%20%28single-precision%29)))

(fn ConstructionScript
  (Utilities|FlowControl|Sequence
    (:then_0
      (switch Utilities|FlowControl|Switch|SwitchonE_VRHandType (Variables|Default|GetHandType)
        (:NewEnumerator0
          (Transformation|SetRelativeScale3D (Variables|Default|GetHandMesh) "1.000000,1.000000,1.000000"))
        (:NewEnumerator1
          (Transformation|SetRelativeScale3D (Variables|Default|GetHandMesh) "1.000000,-1.000000,1.000000")
          (Transformation|SetRelativeTransform (Variables|Default|GetHandRoot) (Math|Transform|MakeTransform (LocalVariables|GetLeftHandOffset) (LocalVariables|GetLeftHandRot) "1,1,1") false false)
          (Rendering|SetVisibility (Variables|Default|Getleft_OculusTouch_v3Controller) (Variables|Default|GetbShowPreviewMesh) false)
          (Rendering|SetVisibility (Variables|Default|Getright_OculusTouch_v3Controller) false false)
          (Transformation|SetRelativeTransform (Variables|Default|GetBPC_GrabSrc) (Math|Transform|MakeTransform "0, 0, 0" (LocalVariables|GetLeftGrabRot) "1,1,1") false false))
        (:NewEnumerator2
          (Transformation|SetRelativeScale3D (Variables|Default|GetHandMesh) "1.000000,1.000000,1.000000")
          (Transformation|SetRelativeTransform (Variables|Default|GetHandRoot) (Math|Transform|MakeTransform (LocalVariables|GetRightHandOffset) (LocalVariables|GetRightHandRot) "1,1,1") false false)
          (Rendering|SetVisibility (Variables|Default|Getleft_OculusTouch_v3Controller) false false)
          (Rendering|SetVisibility (Variables|Default|Getright_OculusTouch_v3Controller) (Variables|Default|GetbShowPreviewMesh) false)
          (Transformation|SetRelativeTransform (Variables|Default|GetBPC_GrabSrc) (Math|Transform|MakeTransform "0, 0, 0" "0, 0, 0" "1,1,1") false false))))))

(fn SetFingerData
  (params (FingerData :type F%20Hand%20Pose%20Data%20Structure))
  (Default|UpdateFingerData (CallFunction|GetHandAnimInstance) FingerData))

(fn GetHandAnimInstance
  (bind _asabp_vr_hand (Utilities|Casting|CastToABP_VR_Hand (Components|SkeletalMesh|GetAnimInstance (Variables|Default|GetHandMesh))))
  (return _asabp_vr_hand))