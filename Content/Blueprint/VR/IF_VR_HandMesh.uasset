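; VR hand mesh actor that shows a posed left or right hand, optionally with a controller preview mesh.
; The construction script mirrors the mesh on Y for left hands, picks a ghost or normal material, and offsets the hand per headset from a position data asset.
; Poses come from a data table row, falling back to HandPoseData, and reach the animation instance as whole-hand or per-finger messages.
; BeginPlay reapplies HandPoseData.
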(event EventBeginPlay
  (CallFunction|UpdateHandPose (Variables|Config|GetHand%20Pose%20Data)))

(event Collision|EventActorBeginOverlap
  (params (OtherActor :type Actor%20Object%20Reference)))

(event EventTick
  (params (DeltaSeconds :type Float%20%28single-precision%29)))

(fn ConstructionScript
  (bind _postiondataasset (Variables|Config|GetPostionDataAsset))
  (bind _hmd_type (Variables|Config|GetHMD%20Type))
  (bind _data (Variables|/Script/InteractionFramework.IF_VRHandMeshPositionData|GetData _postiondataasset))
  (bind (_value _returnvalue) (Utilities|Map|Find _data _hmd_type))
  (bind (_location_left _rotation_left _location_right _rotation_right) (Utilities|Struct|BreakIF_VRHandMeshPosition _value))
  (Utilities|FlowControl|Sequence
    (:then_0
      (|HandMeshScale)
      (|GhostMat))
    (:then_1
      (bind _returnvalue_2 (Utilities|GetDataTableRow "/InteractionFramework/Blueprint/Data/DT_HandPoseData.DT_HandPoseData" (Variables|Config|GetHandPoseKey))
        (:then
          (CallFunction|UpdateHandPose _returnvalue_2))
        (:RowNotFound
          (CallFunction|UpdateHandPose (Variables|Config|GetHand%20Pose%20Data)))))
    (:then_2
      (if _returnvalue
        (switch Utilities|FlowControl|Switch|SwitchonEIF_VRHandType (Variables|Config|GetHandType)
          (:Left
            (Transformation|SetRelativeLocationAndRotation (Variables|Default|GetHandRoot) _location_left _rotation_left false false))
          (:Right
            (Transformation|SetRelativeLocationAndRotation (Variables|Default|GetHandRoot) _location_right _rotation_right false false)))))
    (:then_3
      (Rendering|SetVisibility (Variables|Default|Getleft_ValveIndexController) false false)
      (if (Variables|Config|Preview|GetbPreviewDeviceMesh)
        (switch Utilities|FlowControl|Switch|SwitchonEIF_VRHMDType (Variables|Config|GetHMD%20Type)
          (:SteamVR_Vive
            (Rendering|SetVisibility (Variables|Default|GetHTCViveController) true false))
          (:SteamVR_Index
            (switch Utilities|FlowControl|Switch|SwitchonEIF_VRHandType (Variables|Config|GetHandType)
              (:Left
                (Rendering|SetVisibility (Variables|Default|Getleft_ValveIndexController) true false))
              (:Right
                (Rendering|SetVisibility (Variables|Default|Getright_ValveIndexController) true false))))
          (:Meta_Quest
            (switch Utilities|FlowControl|Switch|SwitchonEIF_VRHandType (Variables|Config|GetHandType)
              (:Left
                (Rendering|SetVisibility (Variables|Default|Getleft_OculusTouch_v3Controller) true false))
              (:Right
                (Rendering|SetVisibility (Variables|Default|Getright_OculusTouch_v3Controller) true false)))))))))

(fn UpdateHandPose
  (params (Data :type IF%20VR%20Hand%20Pose%20Data%20Structure))
  (Class|IFHandPoseInterface|UpdateAllFingerData(Message) (Components|SkeletalMesh|GetAnimInstance (Variables|Default|GetMesh)) Data))

(fn UpdateFingerPose
  (params (Data :type IF%20VR%20Hand%20Finger%20Data%20Structure%20%28by%20ref%29) (Finger :type EIF_HandFingerType%20Enum :default "None"))
  (Class|IFHandPoseInterface|UpdateFingerData(Message) (Components|SkeletalMesh|GetAnimInstance (Variables|Default|GetMesh)) Finger Data))