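; Ghost helper actor that builds a translucent look-alike of an Avatar actor and attaches itself to its owner.
; InitGhostHelper recursively mirrors the avatar's component tree, copying child static and skeletal meshes but no mesh for the root, with scene components standing in for other types.
; Mesh copies share one dynamic ghost material, whose opacity the DisapearMatLerp timeline drives when Disapear plays it.
; UpdateTarget only stores a snap target, and the transform easing is unwired.
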(event EventBeginPlay
  (bind _returnvalue (Rendering|Material|CreateDynamicMaterialInstance "/InteractionFramework/Mat/M_IF_Ghost_Inst.M_IF_Ghost_Inst" "None" "None" :!class /Script/Engine.KismetMaterialLibrary))
  (Variables|Default|SetDynamicMat _returnvalue)
  (InteractionFramework|Ghost|SetGhostOpacity (Variables|Default|GetDefaultOpacity)))

(event EventTick
  (params (DeltaSeconds :type Float%20%28single-precision%29)))

(fn ConstructionScript)

(fn AddAvatarRootComp
  (bind _asprimitive_component (Utilities|Casting|CastToPrimitiveComponent (Variables|/Script/Engine.Actor|GetRootComponent (Variables|Default|GetAvatar)))
    (:then
      (Variables|Default|SetbAvatorRootComponentIsSceneComp false)
      (Utilities|Casting|CastToStaticMeshComponent _asprimitive_component
        (:then
          (bind _returnvalue (AddComponent|AddStaticMeshComponent false))
          (Variables|Default|SetLocal%20Root%20Primitive%20Component _returnvalue)
          (CallFunction|SetPrimativeCompGhostMat (Variables|Default|GetLocal%20Root%20Primitive%20Component) :!label _label)
          (Transformation|AttachComponentToComponent (Variables|Default|GetLocal%20Root%20Primitive%20Component) (Variables|Default|GetSnapHelperRoot) "None" "SnapToTarget" "SnapToTarget" "SnapToTarget" true))
        (:CastFailed
          (Utilities|Casting|CastToSkeletalMeshComponent _asprimitive_component
            (:then
              (bind _returnvalue_2 (AddComponent|AddSkeletalMeshComponent false))
              (Variables|Default|SetLocal%20Root%20Primitive%20Component _returnvalue_2)
              (goto _label))
            (:CastFailed
              (Variables|Default|SetbAvatorRootComponentIsSceneComp true :!label _label_2)
              (bind _returnvalue_3 (AddComponent|AddSceneComponent false))
              (bind _output_get (Variables|Default|SetLocal%20Root%20Scene%20Component _returnvalue_3))
              (Transformation|AttachComponentToComponent _output_get (Variables|Default|GetSnapHelperRoot) "None" "SnapToTarget" "SnapToTarget" "SnapToTarget" true))))))
    (:CastFailed
      (goto _label_2))))

(fn AddChildrenComp
  (params (LocalRootComp :type Scene%20Component%20Object%20Reference) (AvatarRootComp :type Scene%20Component%20Object%20Reference) (Level :type Integer))
  (LocalVariables|SetnewLevel (+ Level 1))
  (bind _output_get (LocalVariables|SetNewLocalVar_0 (Components|GetChildrenComponents AvatarRootComp false)))
  (for _array_element _output_get
    (bind _output_get_2 (LocalVariables|SetmAvatarChild _array_element))
    (LocalVariables|SetRelative (Transformation|GetRelativeTransform (LocalVariables|GetmAvatarChild)))
    (bind _asprimitive_component (Utilities|Casting|CastToPrimitiveComponent _output_get_2)
      (:then
        (bind _asstatic_mesh_component (Utilities|Casting|CastToStaticMeshComponent _asprimitive_component)
          (:then
            (bind _returnvalue (AddComponent|AddStaticMeshComponent false))
            (Components|StaticMesh|SetStaticMesh _returnvalue (Variables|/Script/Engine.StaticMeshComponent|GetStaticMesh _asstatic_mesh_component))
            (Utilities|Map|Add (Variables|Components|GetAvatorChildrenSceneComponents) _returnvalue (LocalVariables|GetnewLevel))
            (CallFunction|SetPrimativeCompGhostMat _returnvalue)
            (Transformation|AttachComponentToComponent _returnvalue LocalRootComp "None" "KeepWorld" "KeepWorld" "KeepWorld" true)
            (Transformation|SetRelativeTransform _returnvalue (LocalVariables|GetRelative) false false)
            (CallFunction|AddChildrenComp _returnvalue (LocalVariables|GetmAvatarChild) (LocalVariables|GetnewLevel)))
          (:CastFailed
            (bind _asskeletal_mesh_component (Utilities|Casting|CastToSkeletalMeshComponent _asprimitive_component)
              (:then
                (bind _returnvalue_2 (AddComponent|AddSkeletalMeshComponent false))
                (Class|SkinnedMeshComponent|SetSkeletalMesh _returnvalue_2 (Variables|/Script/Engine.SkinnedMeshComponent|GetSkeletalMesh _asskeletal_mesh_component) true)
                (Utilities|Map|Add (Variables|Components|GetAvatorChildrenSceneComponents) _returnvalue_2 (LocalVariables|GetnewLevel))
                (CallFunction|SetPrimativeCompGhostMat _returnvalue_2)
                (Transformation|AttachComponentToComponent _returnvalue_2 LocalRootComp "None" "KeepWorld" "KeepWorld" "KeepWorld" true)
                (Transformation|SetRelativeTransform _returnvalue_2 (LocalVariables|GetRelative) false false)
                (CallFunction|AddChildrenComp _returnvalue_2 (LocalVariables|GetmAvatarChild) (LocalVariables|GetnewLevel)))
              (:CastFailed
                (bind _returnvalue_3 (AddComponent|AddSceneComponent false :!label _label))
                (Utilities|Map|Add (Variables|Components|GetAvatorChildrenSceneComponents) _returnvalue_3 (LocalVariables|GetnewLevel))
                (Transformation|AttachComponentToComponent _returnvalue_3 LocalRootComp "None" "KeepWorld" "KeepWorld" "KeepWorld" true)
                (Transformation|SetRelativeTransform _returnvalue_3 (LocalVariables|GetRelative) false false)
                (CallFunction|AddChildrenComp _returnvalue_3 (LocalVariables|GetmAvatarChild) (LocalVariables|GetnewLevel)))))))
      (:CastFailed
        (goto _label)))))

(fn SetPrimativeCompGhostMat
  (params (Comp :type Primitive%20Component%20Object%20Reference))
  (Utilities|IsValid Comp
    (:Is%20Valid
      (for _index (range 0 (- (Rendering|Material|GetNumMaterials Comp) 1))
        (Rendering|Material|SetMaterial Comp _index (Variables|Default|GetDynamicMat))))))

(fn GetLocalRootComp
  (if (Variables|Default|GetbAvatorRootComponentIsSceneComp)
    (return (Variables|Default|GetLocal%20Root%20Scene%20Component))
    (else
      (return (Variables|Default|GetLocal%20Root%20Primitive%20Component)))))

(fn MakeChildrenCompsDebugString
  (bind _avatorchildrenscenecomponents (Variables|Components|GetAvatorChildrenSceneComponents))
  (LocalVariables|SetResult "")
  (bind _keys (Utilities|Map|Keys _avatorchildrenscenecomponents))
  (for _array_element _keys
    (LocalVariables|SetLevelString "")
    (for _index (range 0 (.Value (Utilities|Map|Find _avatorchildrenscenecomponents _array_element)))
      (LocalVariables|SetLevelString (Utilities|String|Append (LocalVariables|GetLevelString) "- ")))
    (LocalVariables|SetResult (Utilities|String|Append (LocalVariables|GetResult) (LocalVariables|GetLevelString) " " (Utilities|GetDisplayName _array_element) (Utilities|String|Append "   Parent:  " (Utilities|GetDisplayName (Utilities|Array|Get(acopy) (Class|SceneComponent|GetParentComponents _array_element))) "    ") " 
 
")))
  (return (LocalVariables|GetResult)))

(fn InitGhostHelper
  (params (Avatar :type Actor%20Object%20Reference))
  (bind _output_get (Variables|Default|SetAvatar Avatar))
  (Utilities|IsValid _output_get
    (:Is%20Valid
      (CallFunction|AddAvatarRootComp)
      (CallFunction|AddChildrenComp (CallFunction|GetLocalRootComp) (Variables|/Script/Engine.Actor|GetRootComponent (Variables|Default|GetAvatar)))
      (Transformation|AttachActorToActor (Components|GetOwner) "None" "SnapToTarget" "SnapToTarget" "SnapToTarget" true)
      (if (Variables|Default|GetbDrawDebug)
        (bind _debugstring (CallFunction|MakeChildrenCompsDebugString))
        (Development|PrintString _debugstring true true "(R=0.022381,G=1.000000,B=0.000000,A=1.000000)" 5.0)))))

(fn UpdateTarget
  (params (Target :type BPC%20Ghost%20Target%20Object%20Reference))
  (Variables|Default|SetSnapTarget Target))

(fn Disapear
  (Variables|Default|SetbSnapping false)
  (Components|Timeline|PlayfromStart (Variables|Default|GetDisapearMatLerp)))

(fn SetGhostOpacity
  (params (Value :type Float%20%28single-precision%29))
  (bind _dynamicmat (Variables|Default|GetDynamicMat)
    (:then
      (Rendering|Material|SetScalarParameterValue _dynamicmat "Opacity" Value :!class /Script/Engine.MaterialInstanceDynamic))
    (:else)))