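; BPC_GrabTar is a grab-target scene component that lets its owning actor be grabbed by a source component.
; BeGrab either snaps the owner so this component aligns with the source, or eases it there over a duration on Tick, tracking the source's live transform.
; Both paths then attach the owner to the source and fire OnGrabSuccess.
; BeRelease only fires OnRelease, without detaching.
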(event EventBeginPlay)

(event EventTick
  (params (DeltaSeconds :type Float%20%28single-precision%29))
  (bind _returnvalue (Components|GetOwner))
  (if (Variables|Default|GetbStartGrabDuration)
    (Variables|Default|SetAlpha (Math|Float|Clamp(Float) (+ (Math|Float|SafeDivide DeltaSeconds (Variables|Default|GetDuration)) (Variables|Default|GetAlpha))))
    (Transformation|SetActorLocationAndRotation _returnvalue (.Location (Math|Transform|BreakTransform (Math|Interpolation|Ease (Variables|Config|GetEaseFunction) (Variables|Default|GetAlpha) (Transformation|GetActorTransform _returnvalue) (Math|Transform|ComposeTransforms (Class|KismetMathLibrary|ConvertTransformtoRelative (Transformation|GetWorldTransform) (Transformation|GetActorTransform (Components|GetOwner))) (Transformation|GetWorldTransform (Variables|Default|GetSourceComp))) 2.0))) (.Rotation (Math|Transform|BreakTransform (Math|Interpolation|Ease (Variables|Config|GetEaseFunction) (Variables|Default|GetAlpha) (Transformation|GetActorTransform _returnvalue) (Math|Transform|ComposeTransforms (Class|KismetMathLibrary|ConvertTransformtoRelative (Transformation|GetWorldTransform) (Transformation|GetActorTransform (Components|GetOwner))) (Transformation|GetWorldTransform (Variables|Default|GetSourceComp))) 2.0))))
    (if (>= (Variables|Default|GetAlpha) 1.0)
      (Variables|Default|SetbStartGrabDuration false)
      (Transformation|AttachComponentToComponent (Components|GetOwner) (Variables|Default|GetSourceComp) "None" "KeepWorld" "KeepWorld" "KeepWorld" true)
      (Variables|Default|SetAlpha 0.0)
      (Default|CallOnGrabSuccess self))))

(fn BeGrab
  (params (SourceComp :type Scene%20Component%20Object%20Reference) (Duration :type Float%20%28single-precision%29))
  (if (> Duration 0.0)
    (CallFunction|InternalbeGrabdDuration SourceComp Duration)
    (return true)
    (else
      (CallFunction|InternalbeGrab SourceComp)
      (return true))))

(fn InternalbeGrab
  (params (SourceComp :type Scene%20Component%20Object%20Reference))
  (bind _output_get (LocalVariables|SetSourceComponent SourceComp))
  (LocalVariables|SetGrabTargetRelativeToOwner (Class|KismetMathLibrary|ConvertTransformtoRelative (Transformation|GetWorldTransform) (Transformation|GetActorTransform (Components|GetOwner))))
  (LocalVariables|SetStartSourceTransform (Transformation|GetWorldTransform _output_get))
  (Transformation|SetActorLocationAndRotation (Components|GetOwner) (.Location (Math|Transform|BreakTransform (Math|Transform|ComposeTransforms (LocalVariables|GetGrabTargetRelativeToOwner) (Transformation|GetWorldTransform _output_get)))) (.Rotation (Math|Transform|BreakTransform (Math|Transform|ComposeTransforms (LocalVariables|GetGrabTargetRelativeToOwner) (Transformation|GetWorldTransform _output_get)))))
  (Transformation|AttachComponentToComponent (Components|GetOwner) _output_get "None" "KeepWorld" "KeepWorld" "KeepWorld" true)
  (Default|CallOnGrabSuccess self))

(fn InternalbeGrabdDuration
  (params (SourceComp :type Scene%20Component%20Object%20Reference) (Duration :type Float%20%28single-precision%29))
  (Variables|Default|SetSourceComp SourceComp)
  (Variables|Default|SetDuration Duration)
  (Variables|Default|SetbStartGrabDuration true)
  (Variables|Default|SetAlpha 0.0))

(fn BeRelease
  (Default|CallOnRelease))