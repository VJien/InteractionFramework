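; Snap source component that finds the nearest tagged target near a source socket and snaps its owning actor onto it.
; Targets come from overlap events or per-tick sphere traces, with an optional ghost helper actor notified of target changes.
; Within the auto-snap radius, the owner eases linearly to the target, then attaches and stops checking.
; Most of this logic is unwired from its events and function entries, so it never runs as saved.
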(event Custom|OnBeginOverlap
  (params (OverlappedComponent :type Primitive%20Component%20Object%20Reference) (OtherActor :type Actor%20Object%20Reference) (OtherComp :type Primitive%20Component%20Object%20Reference) (OtherBodyIndex :type Integer) (bFromSweep :type Boolean) (SweepResult :type Hit%20Result%20Structure%20%28by%20ref%29)))

(event Custom|OnEndOverlap
  (params (OverlappedComponent :type Primitive%20Component%20Object%20Reference) (OtherActor :type Actor%20Object%20Reference) (OtherComp :type Primitive%20Component%20Object%20Reference) (OtherBodyIndex :type Integer)))

(event EventBeginPlay
  (Variables|Private|SetbCheck (Variables|Config|GetbAutoCheck)))

(event EventTick
  (params (DeltaSeconds :type Float%20%28single-precision%29))
  (if (Variables|Private|GetbCheck)
    _))

(fn Init
  (params (SourceComponent :type Primitive%20Component%20Object%20Reference) (Socket :type Name)))

(fn SnaptoNearestTarget
  (Variables|Private|SetStartPosition (Transformation|GetActorTransform (Variables|Private|GetOwnerActor)))
  (Variables|Private|SetAlpha 0.0)
  (Variables|Private|SetbSnapTo true))

(fn CalcNearestTargetComp
  (params (Array :type Array%20of%20%20Object%20References)))

(fn OnGhostSnapEnd)

(fn CalcNearestCompMultiTrace
  (params (Array :type Array%20of%20Hit%20Result%20Structures)))

(fn CheckandSetTarget
  (params (NearestTargetComp :type %20Object%20Reference)))

(fn EnableCheck
  (params (bCheck :type Boolean))
  (Variables|Private|SetbCheck bCheck))